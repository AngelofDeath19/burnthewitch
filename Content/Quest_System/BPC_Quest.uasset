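; Quest component that tracks the active quest's kill-enemy and open-chest objectives and drives the quest HUD.
; It creates WB_QuestHUD at BeginPlay, hides the panel, and fills it with the quest name and objectives through separate events.
; EliminateEnemy shrinks a working array of target actors, while OpenChest matches the chest reference.
; Finished objectives update the HUD and a counter that clears the quest and plays the completion animation when all are done.
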(event `self.ReceiveBeginPlay`
  (bind _returnvalue (`|CreateWidget` "/Game/Quest_System/WB_QuestHUD.WB_QuestHUD_C"))
  (bind _output_get (set `self.Quest HUD Widget` _returnvalue))
  (`UserWidget.AddToViewport` _output_get 0)
  (`/Game/Quest_System/WB_QuestHUD.Hide Quest Pannel` (`self.Quest HUD Widget`)))

(event `Set Active Quset Text`
  (`TextBlock.SetText` (`/Game/Quest_System/WB_QuestHUD.ActiveQuestText` (`self.Quest HUD Widget`)) (`KismetTextLibrary.Conv_StringToText` (`.Name_2_6130ECAD4550EEC7F6E6BF87A5CCD998` (break `/Game/Quest_System/S_Quest` (`self.activeQuest`)))))
  (`/Game/Quest_System/WB_QuestHUD.Show Quest Panel` (`self.Quest HUD Widget`)))

(event `Set Objectives`
  (bind (_activequest_name _activequest_description _activequest_secondary _activequest_completed _activequest_objectives) (break `/Game/Quest_System/S_Quest` (`self.activeQuest`)))
  (`/Game/Quest_System/WB_QuestHUD.Fill Objectives` (`self.Quest HUD Widget`) _activequest_objectives))

(event `Eliminate Enemy`
  (params (`Enemy Eliminating` :type "Actor Object Reference"))
  (bind (_activequest_name _activequest_description _activequest_secondary _activequest_completed _activequest_objectives) (break `/Game/Quest_System/S_Quest` (`self.activeQuest`)))
  (bind _returnvalue (`KismetArrayLibrary.Array_Length` (`self.Enemy Actors Array`)))
  (for _array_element _activequest_objectives
    (bind (_nameaim _completed _actorstoeliminate _chesttoopen _iseliminateenemyobjective _ischestobjective) (break `/Game/Quest_System/S_QuestObjective` _array_element))
    (if (and (not _completed) _iseliminateenemyobjective)
      (if (not (!= (`KismetArrayLibrary.Array_Length` (`self.Enemy Actors Array`)) 0))
        (bind _output_get (set `self.Enemy Actors Array` _actorstoeliminate)))
      (`KismetArrayLibrary.Array_RemoveItem` _output_get `Enemy Eliminating`)
      (`|VariableSetRef` _array_element (make `/Game/Quest_System/S_QuestObjective` _nameaim false (`self.Enemy Actors Array`) _chesttoopen _iseliminateenemyobjective _ischestobjective))
      (`KismetSystemLibrary.PrintString` (`KismetStringLibrary.Conv_IntToString` _returnvalue))
      (if (== _returnvalue 0)
        (`|VariableSetRef` _array_element (make `/Game/Quest_System/S_QuestObjective` _nameaim true _ _chesttoopen _iseliminateenemyobjective _ischestobjective))
        (`/Game/Quest_System/WB_QuestHUD.Complete Objective` (`self.Quest HUD Widget`) _array_element)
        (`self.Objective Completed`)))))

(event `Open Chest`
  (params (Chest :type "Actor Object Reference"))
  (bind (_activequest_name _activequest_description _activequest_secondary _activequest_completed _activequest_objectives) (break `/Game/Quest_System/S_Quest` (`self.activeQuest`)))
  (for _array_element _activequest_objectives
    (bind (_nameaim _completed _actorstoeliminate _chesttoopen _iseliminateenemyobjective _ischestobjective) (break `/Game/Quest_System/S_QuestObjective` _array_element))
    (if (and _ischestobjective (== Chest _chesttoopen))
      (`|VariableSetRef` _array_element (make `/Game/Quest_System/S_QuestObjective` _nameaim false _actorstoeliminate null _iseliminateenemyobjective _ischestobjective))
      (`/Game/Quest_System/WB_QuestHUD.Complete Objective` (`self.Quest HUD Widget`) _array_element)
      (`self.Objective Completed`))))

(event `Objective Completed`
  (bind (_activequest_name _activequest_description _activequest_secondary _activequest_completed _activequest_objectives) (break `/Game/Quest_System/S_Quest` (`self.activeQuest`)))
  (`/Engine/EditorBlueprintResources/StandardMacros.IncrementInt` (`self.objectivesCompleted`)
    (:`  `
      (if (== (`KismetArrayLibrary.Array_Length` _activequest_objectives) (`self.objectivesCompleted`))
        (`/Game/Quest_System/WB_QuestHUD.Complete Objective` :`self` (`self.Quest HUD Widget`))
        (`self.Objective Completed`)
        (`KismetSystemLibrary.PrintString` "Completed")
        (set `self.activeQuest` (struct))
        (set `self.objectivesCompleted` 0)
        (`/Game/Quest_System/WB_QuestHUD.Play Quest Completed Animation` (`self.Quest HUD Widget`))))))